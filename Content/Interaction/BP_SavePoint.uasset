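; BP_SavePoint is an interactable save point that writes the game and lights a fire effect when used.
; Interact sets the FireActive flag, saves through CGameMode's WriteSaveGame, prints a debug message, then calls FireActive.
; FireActive activates the particle system if the flag is set, and OnActorLoaded calls it again to restore the lit state after loading.
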(event Custom|FireActive
  (if (Variables|Default|GetbFireActive)
    (Components|Activation|Activate (Variables|Default|GetParticleSystem) false)))

(event EventInteract
  (params (InstigatorPawn :type Pawn%20Object%20Reference))
  (Variables|Default|SetbFireActive true)
  (bind _ascgame_mode (Utilities|Casting|CastToCGameMode (Game|GetGameMode)))
  (Class|CGameMode|WriteSaveGame _ascgame_mode)
  (Development|PrintString "Saved Game on SavePoint")
  (CallFunction|FireActive))

(event EventOnActorLoaded
  (CallFunction|FireActive))

(fn ConstructionScript)